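; BP_RegistryOpt is a self-test for Windows registry read and write functions.
; On BeginPlay it writes DWORD, QWORD, string, expandable string and multi-string values under its configured Category and Path.
; It reads each back, prints normal or abnormal in Chinese after comparing with the source variable, then deletes all test values.
; A disconnected snippet would print NVIDIA's ShowDlssIndicator value from LocalMachine.
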(event `self.ReceiveBeginPlay`
  (bind _category (`self.Category`))
  (bind _path (`self.Path`))
  (bind _path_2 (`self.Path`))
  (bind _category_2 (`self.Category`))
  (`RegistryOptWindowsBPLibrary.TrySetDwordValue` _category _path "DwKey" (`self.DwKey`))
  (`RegistryOptWindowsBPLibrary.TrySetQwordValue` _category _path "QwKey" (`self.QwKey`))
  (`RegistryOptWindowsBPLibrary.TrySetStringValue` _category _path "SzKey" (`self.SzKey`))
  (`RegistryOptWindowsBPLibrary.TrySetExpandStringValue` _category _path "SzExpandKey" (`self.SzExpandKey`))
  (`RegistryOptWindowsBPLibrary.TrySetMultiStringValue` _category _path "SzMultiKey" (`self.SzMultiKey`))
  (bind _returnvalue (`RegistryOptWindowsBPLibrary.GetDwordValue` (`self.Category`) (`self.Path`) "DwKey"))
  (if (== (`KismetStringLibrary.Conv_StringToInt` _returnvalue) (`self.DwKey`))
    (`KismetSystemLibrary.PrintString` "Dword 正常")
    (else
      (`KismetSystemLibrary.PrintString` "Dword 异常")))
  (bind _returnvalue_2 (`RegistryOptWindowsBPLibrary.GetQwordValue` (`self.Category`) (`self.Path`) "QwKey"))
  (if (== (`KismetStringLibrary.Conv_StringToInt` _returnvalue_2) (`self.QwKey`))
    (`KismetSystemLibrary.PrintString` "Qword 正常")
    (else
      (`KismetSystemLibrary.PrintString` "Qword 异常")))
  (bind _returnvalue_3 (`RegistryOptWindowsBPLibrary.GetStringValue` (`self.Category`) (`self.Path`) "SzKey"))
  (if (`KismetStringLibrary.EqualEqual_StrStr` _returnvalue_3 (`self.SzKey`))
    (`KismetSystemLibrary.PrintString` "String 正常")
    (else
      (`KismetSystemLibrary.PrintString` "String 异常")))
  (bind _returnvalue_4 (`RegistryOptWindowsBPLibrary.GetExpandStringValue` (`self.Category`) (`self.Path`) "SzExpandKey"))
  (if (`KismetStringLibrary.EqualEqual_StrStr` _returnvalue_4 (`self.SzExpandKey`))
    (`KismetSystemLibrary.PrintString` "StringExpand 正常")
    (else
      (`KismetSystemLibrary.PrintString` "StringExpand 异常")))
  (bind _returnvalue_5 (`RegistryOptWindowsBPLibrary.TryGetMultiStringValue` (`self.Category`) (`self.Path`) "SzMultiKey"))
  (if (`KismetArrayLibrary.Array_Identical` _returnvalue_5 (`self.SzMultiKey`))
    (`KismetSystemLibrary.PrintString` "StringMulti 正常")
    (else
      (`KismetSystemLibrary.PrintString` "StringMulti 异常")))
  (`RegistryOptWindowsBPLibrary.DeleteRegistryValue` _category_2 _path_2 "DwKey")
  (`RegistryOptWindowsBPLibrary.DeleteRegistryValue` _category_2 _path_2 "QwKey")
  (`RegistryOptWindowsBPLibrary.DeleteRegistryValue` _category_2 _path_2 "SzKey")
  (`RegistryOptWindowsBPLibrary.DeleteRegistryValue` _category_2 _path_2 "SzExpandKey")
  (`RegistryOptWindowsBPLibrary.DeleteRegistryValue` _category_2 _path_2 "SzMultiKey"))

(fn `UserConstructionScript`)